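; Game mode Blueprint that shows the start-game and game-over UI.
; The StartGame event creates WBP_StartGameWidget and adds it to the viewport.
; The GameOver event adds WBP_GameOverWidget, then uses its WonGame flag to set the WinLose text to a green win or red loss message.
; Neither event is called within this Blueprint, and it holds no other game rules.
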(event `self.StartGame`
  (bind _returnvalue (`|CreateWidget` "/Game/Blueprints/Widgets/WBP_StartGameWidget.WBP_StartGameWidget_C"))
  (`UserWidget.AddToViewport` _returnvalue 0))

(event `self.GameOver`
  (params (bWonGame :type Boolean))
  (bind _returnvalue (`|CreateWidget` "/Game/Blueprints/Widgets/WBP_GameOverWidget.WBP_GameOverWidget_C"))
  (`UserWidget.AddToViewport` _returnvalue 0)
  (if bWonGame
    (bind _winlose (`/Game/Blueprints/Widgets/WBP_GameOverWidget.WinLose` _returnvalue))
    (`TextBlock.SetText` _winlose "You Won!")
    (`TextBlock.SetColorAndOpacity` _winlose (make `SlateColor` (struct :`R` 0.111207 :`G` 0.510417 :`A` 1.0)))
    (else
      (`TextBlock.SetText` _winlose "You Lost!")
      (`TextBlock.SetColorAndOpacity` _winlose (make `SlateColor` (struct :`R` 0.546875 :`G` 0.01362 :`A` 1.0))))))

(fn `UserConstructionScript`)