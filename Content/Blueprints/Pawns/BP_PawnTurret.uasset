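; BP_PawnTurret is a turret pawn Blueprint that displays its health on two widget health bars.
; Each tick, it casts the widgets of Widget and Widget1 to WBP_HealthWidget and sets each HealthBar percent from the Health component's current-to-maximum ratio.
; The updates poll every frame, and a failed cast on the first widget also skips the second.
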(event `self.ReceiveTick`
  (params (DeltaSeconds :type "Float (single-precision)"))
  (bind _health (`self.Health`))
  (bind _health_2 (`self.Health`))
  (bind _aswbp_health_widget (cast `/Game/Blueprints/Widgets/WBP_HealthWidget` (`WidgetComponent.GetWidget` (`self.Widget`))))
  (`ProgressBar.SetPercent` (`/Game/Blueprints/Widgets/WBP_HealthWidget.HealthBar` _aswbp_health_widget) (/ (`HealthComponent.Health` _health) (`HealthComponent.MaxHealth` _health)))
  (bind _aswbp_health_widget_2 (cast `/Game/Blueprints/Widgets/WBP_HealthWidget` (`WidgetComponent.GetWidget` (`self.Widget1`))))
  (`ProgressBar.SetPercent` (`/Game/Blueprints/Widgets/WBP_HealthWidget.HealthBar` _aswbp_health_widget_2) (/ (`HealthComponent.Health` _health_2) (`HealthComponent.MaxHealth` _health_2))))

(fn `UserConstructionScript`)